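; BP_Key is a key pickup that the BP_Girl character collects by pressing K while in range.
; Overlapping its Collision component enables input on the key for the girl's PlayerController, and ending the overlap disables it.
; Pressing K fires the KeyIsTakenTrigger event dispatcher to signal the pickup, then destroys the key actor.
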(event OnComponentBeginOverlap(collision)
  (params (OverlappedComponent :type Primitive%20Component%20Object%20Reference) (OtherActor :type Actor%20Object%20Reference) (OtherComp :type Primitive%20Component%20Object%20Reference) (OtherBodyIndex :type Integer) (bFromSweep :type Boolean) (SweepResult :type Hit%20Result%20Structure%20%28by%20ref%29))
  (bind _asbp_girl (Utilities|Casting|CastToBP_Girl OtherActor))
  (bind _asplayer_controller (Utilities|Casting|CastToPlayerController (Pawn|GetController _asbp_girl)))
  (Input|EnableInput _asplayer_controller))

(event OnComponentEndOverlap(collision)
  (params (OverlappedComponent :type Primitive%20Component%20Object%20Reference) (OtherActor :type Actor%20Object%20Reference) (OtherComp :type Primitive%20Component%20Object%20Reference) (OtherBodyIndex :type Integer))
  (bind _asbp_girl (Utilities|Casting|CastToBP_Girl OtherActor))
  (bind _asplayer_controller (Utilities|Casting|CastToPlayerController (Pawn|GetController _asbp_girl)))
  (Input|DisableInput _asplayer_controller))

(event EventBeginPlay)

(event EventTick
  (params (DeltaSeconds :type Float%20%28single-precision%29)))

(event Input|KeyboardEvents|K
  (params (Key :type Key%20Structure))
  (:Pressed
    (Default|CallKeyIsTakenTrigger)
    (Actor|DestroyActor)))

(fn ConstructionScript)