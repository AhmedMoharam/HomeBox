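; BP_Box is an interactive box whose cover opens once when the player presses E nearby.
; When BP_Girl overlaps BoxTriggerVolume, it shows BoxText and enables input on the box, reversing both when she leaves.
; If CanBeOpened is set, E fires OpenBox through a DoOnce, where a timeline drives the cover's world pitch, then calls the BoxIsOpenedTrigger dispatcher on finish.
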(event OnComponentBeginOverlap(BoxTriggerVolume)
  (params (OverlappedComponent :type Primitive%20Component%20Object%20Reference) (OtherActor :type Actor%20Object%20Reference) (OtherComp :type Primitive%20Component%20Object%20Reference) (OtherBodyIndex :type Integer) (bFromSweep :type Boolean) (SweepResult :type Hit%20Result%20Structure%20%28by%20ref%29))
  (Utilities|Casting|CastToBP_Girl OtherActor)
  (CallFunction|ShowText)
  (Input|EnableInput (Game|GetPlayerController 0)))

(event OnComponentEndOverlap(BoxTriggerVolume)
  (params (OverlappedComponent :type Primitive%20Component%20Object%20Reference) (OtherActor :type Actor%20Object%20Reference) (OtherComp :type Primitive%20Component%20Object%20Reference) (OtherBodyIndex :type Integer))
  (Utilities|Casting|CastToBP_Girl OtherActor)
  (CallFunction|HideText)
  (Input|DisableInput (Game|GetPlayerController 0)))

(event Custom|OpenBox
  (bind _boxcover (Variables|Default|GetBoxCover))
  (bind _returnvalue (Transformation|GetWorldRotation _boxcover))
  (bind _angle (Timeline|Timeline_0 Play)
    (:Update
      (Transformation|SetWorldRotation _boxcover (Math|Rotator|MakeRotator (.roll _returnvalue) _angle (.yaw _returnvalue)) false false))
    (:Finished
      (Default|CallBoxIsOpenedTrigger))))

(event EventBeginPlay)

(event Input|KeyboardEvents|E
  (params (Key :type Key%20Structure))
  (:Pressed
    (if (Variables|Default|GetCanBeOpened?)
      (Utilities|FlowControl|DoOnce false
        (:Completed
          (CallFunction|OpenBox))))))

(fn ConstructionScript)

(fn ShowText
  (Rendering|SetVisibility (Variables|Default|GetBoxText) true false))

(fn HideText
  (Rendering|SetVisibility (Variables|Default|GetBoxText) false false))