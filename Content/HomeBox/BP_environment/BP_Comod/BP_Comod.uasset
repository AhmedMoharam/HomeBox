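; BP_Comod is an interactive commode with a drawer that the player opens and closes with E.
; Overlap by BP_Girl shows the commode text, hides the guide widget and enables input; leaving hides the text and disables input.
; If CanBeOpened is set, E alternates two timelines via FlipFlop, adding local X offsets to the drawer each update.
; Each timeline's completion updates IsOpened and calls the matching opened or closed trigger.
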(event OnComponentBeginOverlap(TriggerBox)
  (params (OverlappedComponent :type Primitive%20Component%20Object%20Reference) (OtherActor :type Actor%20Object%20Reference) (OtherComp :type Primitive%20Component%20Object%20Reference) (OtherBodyIndex :type Integer) (bFromSweep :type Boolean) (SweepResult :type Hit%20Result%20Structure%20%28by%20ref%29))
  (Utilities|Casting|CastToBP_Girl OtherActor)
  (CallFunction|HideUIwiget)
  (CallFunction|ShowText)
  (Input|EnableInput (Game|GetPlayerController 0)))

(event OnComponentEndOverlap(TriggerBox)
  (params (OverlappedComponent :type Primitive%20Component%20Object%20Reference) (OtherActor :type Actor%20Object%20Reference) (OtherComp :type Primitive%20Component%20Object%20Reference) (OtherBodyIndex :type Integer))
  (Utilities|Casting|CastToBP_Girl OtherActor)
  (CallFunction|HideText)
  (Input|DisableInput (Game|GetPlayerController 0)))

(event Custom|Open/CloseComode
  ;[1 1 1] Open/Close Comode
  (Utilities|FlowControl|FlipFlop
    (:A
      (bind _drawerxpostion (Timeline|OpenComodeTimeline PlayFromStart)
        (:Update
          (Transformation|AddLocalOffset (Variables|Default|GetDrawer) (Math|Vector|MakeVector _drawerxpostion 0.0 0.0) false false))
        (:Finished
          (Variables|Default|SetIsOpened? true)
          (Default|CallComodeIsOpenedTrigger))))
    (:B
      (bind _drawerxpostion_2 (Timeline|Timeline_0 PlayFromStart)
        (:Update
          (Transformation|AddLocalOffset (Variables|Default|GetDrawer) (Math|Vector|MakeVector (* -1 _drawerxpostion_2) 0.0 0.0) false false))
        (:Finished
          (Variables|Default|SetIsOpened? false)
          (Default|CallComodeIsClosedTrigger))))))

(event Input|KeyboardEvents|E
  (params (Key :type Key%20Structure))
  ;[1 1 1] Open/Close Comode
  (:Pressed
    (if (Variables|Default|GetCanBeOpened?)
      (CallFunction|Open/CloseComode))))

(fn ConstructionScript)

(fn HideUIwiget
  (Rendering|SetVisibility (Variables|Default|GetUIwidgetGuide) false false))

(fn ShowUIwidget
  (Rendering|SetVisibility (Variables|Default|GetUIwidgetGuide) true false))

(fn ShowText
  (Rendering|SetVisibility (Variables|Default|GetComodeText) true false))

(fn HideText
  (Rendering|SetVisibility (Variables|Default|GetComodeText) false false))