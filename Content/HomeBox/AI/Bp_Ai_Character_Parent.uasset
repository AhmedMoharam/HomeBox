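; Parent AI character Blueprint that patrols target actors until it sees the girl character, then chases her.
; A looping timer moves it along the Targets array, bouncing between the last two once it reaches the end.
; Pawn sensing clears that timer and starts a repeating chase timer once, with no return to patrol.
; Catch results are only debug prints, and a separate catch graph duplicates the chase move.
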(event OnSeePawn(PawnSensing)
  (params (Pawn :type Pawn%20Object%20Reference))
  (bind _asbp_girl (Utilities|Casting|CastToBP_Girl Pawn))
  (Development|PrintString "i saw u Muaahaha")
  (Utilities|Time|ClearandInvalidateTimerbyHandle (Variables|Default|GetPatrolling))
  (if (not (Variables|Default|GetCatchingFunctionCreated))
    (bind _returnvalue (Utilities|Time|SetTimerbyFunctionName self "CatchThePlayer" 2.0 true))
    (Variables|Default|SetCatchThePlayerHandling _returnvalue)
    (Variables|Default|SetCatchingFunctionCreated true)))

(event Custom|Patrol
  (bind _targets (Variables|Default|GetTargets))
  (bind _output_get (Variables|Default|SetLastIndex (- (Utilities|Array|Length _targets) 1)))
  (if (== (Variables|Default|GetTarget%20index) _output_get)
    (Variables|Default|SetTarget%20index (- (Variables|Default|GetTarget%20index) 1))
    (AI|AIMoveTo self "0, 0, 0" (Utilities|Array|Get(acopy) _targets (Variables|Default|GetTarget%20index)) 5.0 false)
    (else
      (Variables|Default|SetTarget%20index (+ (Variables|Default|GetTarget%20index) 1))
      (AI|AIMoveTo self "0, 0, 0" (Utilities|Array|Get(acopy) _targets (Variables|Default|GetTarget%20index)) 5.0 false))))

(event Custom|CatchThePlayer
  (Development|PrintString "I'm Going to u")
  (AI|AIMoveTo self "0, 0, 0" (stale OnSeePawn(PawnSensing) _asbp_girl) 5.0 false
    (:OnSuccess
      (Development|PrintString " i catch u hahah"))
    (:OnFail
      (Development|PrintString "i miss u"))))

(event EventBeginPlay
  (bind _returnvalue (Utilities|Time|SetTimerbyFunctionName self "Patrol" 5.0 true))
  (Variables|Default|SetPatrolling _returnvalue))

(fn ConstructionScript)